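; BP_AiMoveTo is an AI pawn Blueprint that repeatedly moves toward the first player.
; On BeginPlay it runs AI MoveTo with player controller 0 as the target actor, retrying after a short delay on success or failure.
; A separate IsObservable function, not called here, uses a dot product against control rotation to test whether the player faces a given target within a view cone, without an occlusion check.
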(event EventBeginPlay
  (AI|AIMoveTo self "0, 0, 0" (Game|GetPlayerController 0) 2e+02 false :!label _label
    (:OnSuccess
      _)
    (:OnFail
      _))
  (Utilities|FlowControl|Delay 1.0)
  (goto _label))

(fn ConstructionScript)

(fn IsObservable
  (params (Target :type Actor%20Object%20Reference))
  (return (>= (* (Math|Vector|DotProduct (Math|Vector|GetForwardVector (Math|Rotator|FindLookatRotation (Transformation|GetActorLocation Target) (Transformation|GetActorLocation (Game|Player|GetPlayerPawn 0)))) (Math|Vector|GetForwardVector (Pawn|GetControlRotation (Game|GetPlayerCharacter 0) :!class /Script/Engine.Pawn))) -1.0) 0.7)))