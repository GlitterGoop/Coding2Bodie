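; BP_Jumper is a holdable item with primary and secondary use actions.
; Pickup snaps it to the hand_r socket of the given skeletal mesh and disables its Box collision.
; Primary use prints "Throw!" and sets the actor location to a fixed point, with no physics throw.
; Secondary use alternates the Sphere material between flat blue and pink through a FlipFlop.
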(event EventPickup
  (params (SkeletalMesh :type Skeletal%20Mesh%20Component%20Object%20Reference))
  (Transformation|AttachComponentToComponent SkeletalMesh "hand_r" "SnapToTarget" "SnapToTarget" "SnapToTarget" true)
  (Collision|SetCollisionEnabled (Variables|Default|GetBox) "NoCollision"))

(event EventUsePrimary
  (Development|PrintText "Throw!")
  (Transformation|SetActorLocation "0.000000,0.000000,100.000000" false false))

(event EventUseSecondary
  (bind _sphere (Variables|Default|GetSphere))
  (Utilities|FlowControl|FlipFlop
    (:A
      (Rendering|Material|SetMaterial _sphere 0 "/Game/Materials/MI_FlatBlue.MI_FlatBlue"))
    (:B
      (Rendering|Material|SetMaterial _sphere 0 "/Game/Materials/MI_FlatPink.MI_FlatPink"))))

(fn ConstructionScript)