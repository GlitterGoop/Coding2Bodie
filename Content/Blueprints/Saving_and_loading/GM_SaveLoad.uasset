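; GM_SaveLoad is a game mode that persists per-level state, such as collected coins, in an SG_LevelState save object.
; On BeginPlay it loads the slot named after the current level, or creates a fresh save object if none exists.
; After loading, it calls CollectThyself on each valid saved coin, skipping invalid references.
; A separate event writes the save object back to that level's slot and prints the result.
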(event Custom|Save%20LevelState%20to%20File
  (bind _returnvalue (Game|GetCurrentLevelName true))
  (bind _returnvalue_2 (SaveGame|SaveGametoSlot (Variables|Default|GetSG_LevelState) _returnvalue))
  (if _returnvalue_2
    (Development|PrintText "Level state saved" true true "(R=0.114008,G=0.365217,B=0.066597,A=1.000000)" 1e+01)
    (else
      (Development|PrintText "level state failed to save" true true "(R=1.000000,G=0.037400,B=0.069874,A=1.000000)" 5.0))))

(event Custom|Load%20LevelState%20from%20file
  (bind _returnvalue (Game|GetCurrentLevelName true))
  (bind _returnvalue_2 (SaveGame|DoesSaveGameExist _returnvalue))
  (if _returnvalue_2
    (bind _returnvalue_3 (SaveGame|LoadGamefromSlot _returnvalue))
    (bind _assg_level_state (Utilities|Casting|CastToSG_LevelState _returnvalue_3))
    (Variables|Default|SetSG_LevelState _assg_level_state)
    ;[0.15 0.15 0.15 0.5] Load collected coins
    (for _array_element (Variables|/Game/Blueprints/Saving_and_loading/SG_LevelState.SG_LevelState_C|GetCollectedCoins (Variables|Default|GetSG_LevelState))
      (Utilities|IsValid _array_element ; So coins from other levels don't make this crash
        (:Is%20Valid
          (Default|CollectThyself _array_element))))
    (else
      (bind _returnvalue_4 (SaveGame|CreateSaveGameObject "/Game/Blueprints/Saving_and_loading/SG_LevelState.SG_LevelState_C"))
      (Variables|Default|SetSG_LevelState _returnvalue_4))))

(event EventBeginPlay
  (CallFunction|LoadLevelStatefromFile))

(event EventTick
  (params (DeltaSeconds :type Float%20%28single-precision%29)))

(fn ConstructionScript)