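; BP_OtherItem3 is a held item that can be picked up and has primary and secondary use actions.
; Pickup attaches it to the given skeletal mesh's hand_r socket and disables collision on its Box.
; Primary use flip-flops the Sphere component's static mesh between a cowboy bean and a prototype sword.
; Secondary use plays a coin-collect sound at the world origin rather than at the item.
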(event EventPickup
  (params (SkeletalMesh :type Skeletal%20Mesh%20Component%20Object%20Reference))
  (Transformation|AttachComponentToComponent SkeletalMesh "hand_r" "SnapToTarget" "SnapToTarget" "SnapToTarget" true)
  (Collision|SetCollisionEnabled (Variables|Default|GetBox) "NoCollision"))

(event EventUsePrimary
  (Utilities|FlowControl|FlipFlop
    (:A
      (Components|StaticMesh|SetStaticMesh (Variables|Default|GetSphere) "/Game/PolygonStarter/Models/SM_Bean_Cowboy_01.SM_Bean_Cowboy_01"))
    (:B
      (Components|StaticMesh|SetStaticMesh (Variables|Default|GetSphere) "/Game/PolygonStarter/Models/SM_PolygonPrototype_Prop_Sword_01.SM_PolygonPrototype_Prop_Sword_01"))))

(event EventUseSecondary
  (Audio|PlaySoundatLocation "/Game/Audio/collectcoin-6075.collectcoin-6075" "0, 0, 0" "0, 0, 0" 1.0 1.0 0.0 0 0 0 0))

(fn ConstructionScript)