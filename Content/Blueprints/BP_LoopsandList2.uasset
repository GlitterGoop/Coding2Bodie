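; BP_LoopsandList2 is a Blueprint that demonstrates loop types and array indexing through printed on-screen text.
; From BeginPlay, DelayLoop prints its run count, waits briefly, then passes a DoN gate that fires StartForLoop and re-calls DelayLoop until the limit.
; StartForLoop prints indices colored from an array literal.
; ForEach and While variants exist but are never called, and the While condition is fixed false.
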(event Custom|DelayLoop
  (Development|PrintText (Utilities|Text|FormatText "This had run {count} times" (stale _counter)))
  (Utilities|FlowControl|Delay 0.1)
  (bind _counter (Utilities|FlowControl|DoN 20)
    (:Exit
      (CallFunction|StartforLoop)
      (CallFunction|DelayLoop))))

(event Custom|StartForLoop
  (bind _array (Utilities|Array|MakeArray "(R=1.000000,G=0.777002,B=0.086400,A=1.000000)" "(R=1.000000,G=0.156880,B=0.051600,A=1.000000)" "(R=0.129700,G=1.000000,B=0.136719,A=1.000000)" "(R=0.473881,G=0.166170,B=1.000000,A=1.000000)" "(R=0.156270,G=0.519359,B=1.000000,A=1.000000)"))
  (for _index (range 0 (- (Utilities|Array|Length _array) 0) 2)
    (Development|PrintText (Utilities|Text|FormatText "This is index #{index}" _index) true true (Utilities|Array|Get(acopy) _array _index) 0.1)))

(event Custom|StartWhileLoop
  (while false
    (Development|PrintText (Utilities|Text|FormatText "There are {uses} more uses in this loop" (Variables|Default|GetWhileLoopCounter)) true true "(R=1.000000,G=0.073998,B=0.725267,A=1.000000)")
    (Math|Integer|DecrementInt (Variables|Default|GetWhileLoopCounter)))
  (Variables|Default|SetWhileLoopCounter 10))

(event Custom|StartForEachLoop
  (for (_array_element _array_index) (Utilities|Array|MakeArray "(R=1.000000,G=0.777002,B=0.086400,A=1.000000)" "(R=1.000000,G=0.156880,B=0.051600,A=1.000000)" "(R=0.129700,G=1.000000,B=0.136719,A=1.000000)" "(R=0.473881,G=0.166170,B=1.000000,A=1.000000)" "(R=0.156270,G=0.519359,B=1.000000,A=1.000000)")
    (Development|PrintText (Utilities|Text|FormatText "This is index #{index}" _array_index) true true _array_element 0.2)))

(event EventBeginPlay
  (Development|PrintString "Loop and list bp exists")
  (CallFunction|DelayLoop))

(fn ConstructionScript)