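; BP_SpawnManager populates the level with randomized AI characters at placed spawn points when play begins.
; It gathers every BP_SpawnPoint, prints the count, and gives each point a coin-flip chance to spawn a BP_AiMoveTo owned by that point.
; Each spawned AI gets a random name on its text component, plus a random skeletal mesh and materials drawn from enemy arrays.
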(event EventBeginPlay
  (bind _enemymaterials (Variables|Default|GetEnemyMaterials))
  (bind _outitem (Utilities|Array|Random _enemymaterials))
  (bind _outactors (Actor|GetAllActorsOfClass "/Game/Blueprints/BP_SpawnPoint.BP_SpawnPoint_C"))
  (Development|PrintText (Utilities|Text|FormatText "There are {count} spawn points " (Utilities|Array|Length _outactors)) true true "(R=0.000000,G=0.660000,B=1.000000,A=1.000000)" 5.0)
  (for _array_element _outactors
    (if (Math|Random|RandomBool)
      (bind _returnvalue (Game|SpawnActorfromClass "/Game/AI_Blueprints/BP_AiMoveTo.BP_AiMoveTo_C" (Transformation|GetActorTransform _array_element) "Undefined" "MultiplyWithRoot" _array_element 0))
      (Rendering|Components|TextRender|SetText (Variables|/Game/AI_Blueprints/BP_AiMoveTo.BP_AiMoveTo_C|GetAI%20Name%20Text _returnvalue) (.OutItem (Utilities|Array|Random (Variables|Default|GetEnemyNames))))
      (Rendering|Material|SetMaterial (Variables|/Script/Engine.Character|GetMesh _returnvalue) 0 _outitem)
      (Rendering|Material|SetMaterial (Variables|/Script/Engine.Character|GetMesh _returnvalue) 1 _outitem)
      (Components|SkeletalMesh|SetSkeletalMeshAsset (Variables|/Script/Engine.Character|GetMesh _returnvalue) (.OutItem (Utilities|Array|Random (Variables|Default|GetEnemySkeleton)))))))

(fn ConstructionScript)